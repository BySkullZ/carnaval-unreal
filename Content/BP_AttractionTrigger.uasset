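; Trigger actor for a carnival can-knockdown attraction, running one round from start to win or loss.
; Player overlap switches to the attraction camera, swaps movement for BP_ShootBehaviour and adds a mouse-following crosshair widget.
; A box counts and hides cans and destroys balls; enough cans notifies the game mode, too many balls loses.
; Either outcome restores the player and resets the round; leaving the start trigger re-arms it.
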(event OnComponentBeginOverlap(StartTrigger)
  (params (OverlappedComponent :type Primitive%20Component%20Object%20Reference) (OtherActor :type Actor%20Object%20Reference) (OtherComp :type Primitive%20Component%20Object%20Reference) (OtherBodyIndex :type Integer) (bFromSweep :type Boolean) (SweepResult :type Hit%20Result%20Structure%20%28by%20ref%29))
  (if (Variables|Default|GetCanPlay)
    (bind _asbp_third_person_character (Utilities|Casting|CastToBP_ThirdPersonCharacter OtherActor))
    (Variables|Default|SetTPC _asbp_third_person_character)
    (Game|Player|SetViewTargetwithBlend (Game|GetPlayerController 0) (Components|GetOwner (Variables|Default|GetCamera)) 0.0 "VTBlend_Linear" 0.0 false)
    (Variables|/Game/BP_ShootBehaviour.BP_ShootBehaviour_C|SetCameraAttraction (Actor|GetComponentbyClass (Variables|Default|GetTPC) "/Game/BP_ShootBehaviour.BP_ShootBehaviour_C") (Variables|Default|GetCamera))
    (Components|Activation|SetActive (Actor|GetComponentbyClass (Variables|Default|GetTPC) "/Script/Engine.CharacterMovementComponent") false false)
    (Components|Activation|SetActive (Actor|GetComponentbyClass (Variables|Default|GetTPC) "/Game/BP_ShootBehaviour.BP_ShootBehaviour_C") true false)
    (bind _returnvalue (Game|ConstructObjectfromClass (Game|GetPlayerController 0) "/Game/WB_ChambouleTout.WB_ChambouleTout_C"))
    (UserInterface|Viewport|AddtoViewport _returnvalue 0)
    (Variables|Default|SetCrosshair (Variables|/Game/WB_ChambouleTout.WB_ChambouleTout_C|GetCrosshair _returnvalue))))

(event OnComponentBeginOverlap(Box)
  (params (OverlappedComponent :type Primitive%20Component%20Object%20Reference) (OtherActor :type Actor%20Object%20Reference) (OtherComp :type Primitive%20Component%20Object%20Reference) (OtherBodyIndex :type Integer) (bFromSweep :type Boolean) (SweepResult :type Hit%20Result%20Structure%20%28by%20ref%29))
  (bind _tpc (Variables|Default|GetTPC))
  (if (Variables|Default|GetCanPlay)
    (bind _asbp_can (Utilities|Casting|CastToBP_Can OtherActor)
      (:then
        (Rendering|SetActorHiddenInGame _asbp_can true)
        (bind _result (Math|Integer|IncrementInt (Variables|Default|GetCanCount))
          (:%20%20
            (if (>= _result 10)
              (Development|PrintString "winner")
              (bind _returnvalue (Actor|GetActorOfClass "/Game/BP_CarnavalGameMode.BP_CarnavalGameMode_C"))
              (Default|OnEventWinEvent _returnvalue)
              (Variables|Default|SetCanPlay false :!label _label)
              (Components|Activation|SetActive (Actor|GetComponentbyClass _tpc "/Script/Engine.CharacterMovementComponent") true false)
              (Components|Activation|SetActive (Actor|GetComponentbyClass _tpc "/Game/BP_ShootBehaviour.BP_ShootBehaviour_C") false true)
              (Game|Player|SetViewTargetwithBlend (Game|GetPlayerController 0) (Components|GetOwner (Variables|/Game/ThirdPerson/Blueprints/BP_ThirdPersonCharacter.BP_ThirdPersonCharacter_C|GetCameraBoom (Variables|Default|GetTPC))) 0.0 "VTBlend_Linear" 0.0 false)
              (Widget|RemovefromParent (stale OnComponentBeginOverlap(StartTrigger) _returnvalue))
              (CallFunction|ResetCans)))))
      (:CastFailed
        (bind _asbp_ball (Utilities|Casting|CastToBP_Ball OtherActor))
        (Actor|DestroyActor _asbp_ball)
        (bind _result_2 (Math|Integer|IncrementInt (Variables|Default|GetBallCount))
          (:%20%20
            (if (>= _result_2 3)
              (Development|PrintString "lose")
              (goto _label))))))))

(event OnComponentEndOverlap(StartTrigger)
  (params (OverlappedComponent :type Primitive%20Component%20Object%20Reference) (OtherActor :type Actor%20Object%20Reference) (OtherComp :type Primitive%20Component%20Object%20Reference) (OtherBodyIndex :type Integer))
  (Utilities|Casting|CastToBP_ThirdPersonCharacter OtherActor)
  (Variables|Default|SetCanPlay true))

(event Custom|ResetCans
  (Variables|Default|SetCanCount 0)
  (Variables|Default|SetBallCount 0)
  (bind _outactors (Actor|GetAllActorsOfClass "/Game/BP_Can.BP_Can_C"))
  (for _array_element _outactors
    (Default|Reset _array_element)
    (bind _outactors_2 (Actor|GetAllActorsOfClass "/Game/BP_Ball.BP_Ball_C"))
    (for _array_element_2 _outactors_2
      (Actor|DestroyActor _array_element_2))))

(event EventTick
  (params (DeltaSeconds :type Float%20%28single-precision%29))
  (bind _returnvalue (Game|GetPlayerController 0))
  (bind _crosshair (Variables|Default|GetCrosshair))
  (bind (_locationx _locationy) (Game|Player|GetMousePosition _returnvalue))
  (if (Utilities|IsValid _crosshair)
    (Class|CanvasPanelSlot|SetPosition (Class|WidgetLayoutLibrary|SlotasCanvasSlot _crosshair) (Class|SlateBlueprintLibrary|ScreentoViewport (Math|Vector2D|MakeVector2D _locationx _locationy)))))

(fn ConstructionScript)

(fn GetShootedCans
  (return (Variables|Default|GetCanCount)))