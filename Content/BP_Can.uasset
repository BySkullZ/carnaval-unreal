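; BP_Can is a can actor with a physics mesh that can be put back where it started.
; On BeginPlay it stores the static mesh's world transform.
; Its Reset event switches physics simulation off, moves the mesh to the stored transform, switches simulation back on and unhides the actor.
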(event Custom|Reset
  (bind _staticmesh (Variables|Default|GetStaticMesh))
  (Physics|SetSimulatePhysics _staticmesh false)
  (Transformation|SetWorldTransform _staticmesh (Variables|Default|GetInitialPos) false false)
  (Physics|SetSimulatePhysics (Variables|Default|GetStaticMesh) true)
  (Rendering|SetActorHiddenInGame false))

(event EventBeginPlay
  (Variables|Default|SetInitialPos (Transformation|GetWorldTransform (Variables|Default|GetStaticMesh))))

(fn ConstructionScript)