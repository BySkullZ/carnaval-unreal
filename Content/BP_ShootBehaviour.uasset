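; BP_ShootBehaviour is an activatable shooting behaviour, inactive at BeginPlay, that fires charged BP_Ball shots toward the mouse cursor.
; While IA_Shoot triggers, ShootTime eases toward the maximum ImpuseForce through a repeated Lerp.
; On completion, it spawns a ball at CameraAttraction, applies that impulse along the deprojected cursor ray, then resets the charge.
; GetNormalizedShootTime exposes the charge as a clamped 0–1 value.
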(event Input|EnhancedActionEvents|EnhancedInputActionIA_Shoot
  (params (ActionValue :type Boolean) (ElapsedSeconds :type Float%20%28double-precision%29) (TriggeredSeconds :type Float%20%28double-precision%29) (InputAction :type Input%20Action%20Object%20Reference :default "/Game/ThirdPerson/Input/Actions/Character/IA_Shoot.IA_Shoot"))
  (bind _returnvalue (Components|Activation|IsActive))
  (bind _returnvalue_2 (Game|GetPlayerController 0))
  (bind (_locationx _locationy) (Game|Player|GetMousePosition _returnvalue_2))
  (:Triggered
    (if _returnvalue
      (Variables|Default|SetShootTime (Math|Float|Lerp (Variables|Default|GetShootTime) (Variables|Default|GetImpuseForce) 0.01))))
  (:Completed
    (if _returnvalue
      (bind _returnvalue_3 (Game|SpawnActorfromClass "/Game/BP_Ball.BP_Ball_C" (Math|Transform|MakeTransform (Transformation|GetWorldLocation (Variables|Default|GetCameraAttraction))) "Undefined" "MultiplyWithRoot" 0 0))
      (Physics|AddImpulse (Variables|/Game/BP_Ball.BP_Ball_C|GetSphere _returnvalue_3) (* (.WorldDirection (Class|GameplayStatics|DeprojectScreentoWorld _returnvalue_2 (Math|Vector2D|MakeVector2D _locationx _locationy))) (Variables|Default|GetShootTime)) "None" false)
      (Variables|Default|SetShootTime 0.0))))

(event EventBeginPlay
  (Components|Activation|SetActive false false))

(fn GetNormalizedShootTime
  (return (Math|Float|Clamp(Float) (/ (Variables|Default|GetShootTime) (Variables|Default|GetImpuseForce)))))