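; BP_Bumper is a bumper pawn that wanders by AI and also has input handlers for moving and turning.
; AIMove loops AI Move To toward random reachable points around a fixed origin, retrying on success or failure.
; Move input pushes the static mesh with force along the camera's forward vector, while turn input adds world yaw.
; Reset unhides it, restores its BeginPlay transform, stops movement and restarts wandering.
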(event Custom|AI%20Move
  (AI|AIMoveTo self (.RandomLocation (AI|Navigation|GetRandomReachablePointinRadius (Math|Vector|MakeVector -1e+03 0.0 0.0) 5e+02 0 0)) 0 5.0 false
    (:OnSuccess
      _)
    (:OnFail
      _))
  (CallFunction|AIMove self))

(event Custom|Reset
  (Rendering|SetActorHiddenInGame false)
  (Transformation|SetActorTransform (Variables|Default|GetDefaultPos))
  (Components|Movement|StopMovementImmediately (Variables|Default|GetFloatingPawnMovement))
  (CallFunction|AIMove))

(event Input|EnhancedActionEvents|EnhancedInputActionIA_Bumper_Move
  (params (ActionValue :type Float%20%28double-precision%29) (ElapsedSeconds :type Float%20%28double-precision%29) (TriggeredSeconds :type Float%20%28double-precision%29) (InputAction :type Input%20Action%20Object%20Reference :default "/Game/ThirdPerson/Input/Actions/Bumper/IA_Bumper_Move.IA_Bumper_Move"))
  (Physics|AddForce (Variables|Default|GetStaticMesh) (* (* ActionValue (Variables|Default|GetSpeed)) (Math|Vector|ProjectVectorontoPlane (Math|Vector|GetForwardVector (Variables|Default|GetCamera)) "0, 0, 0")) "None" false))

(event Input|EnhancedActionEvents|EnhancedInputActionIA_Bumper_Turn
  (params (ActionValue :type Float%20%28double-precision%29) (ElapsedSeconds :type Float%20%28double-precision%29) (TriggeredSeconds :type Float%20%28double-precision%29) (InputAction :type Input%20Action%20Object%20Reference :default "/Game/ThirdPerson/Input/Actions/Bumper/IA_Bumper_Turn.IA_Bumper_Turn"))
  (Transformation|AddWorldRotation (Variables|Default|GetStaticMesh) (Math|Rotator|MakeRotator 0.0 0.0 (* ActionValue (Variables|Default|GetTurnSpeed))) false false))

(event EventBeginPlay
  (Variables|Default|SetDefaultPos (Transformation|GetActorTransform))
  (CallFunction|AIMove self))

(fn ConstructionScript)